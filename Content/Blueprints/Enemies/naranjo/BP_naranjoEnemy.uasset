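; BP_naranjoEnemy is an enemy Blueprint with health and a simple attack that pauses its movement.
; Attack sets the walk speed to zero, waits two seconds, then restores it; it applies no damage itself.
; DealDamage subtracts incoming damage from HP, prints the remaining value and destroys the actor once HP runs out.
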(event `/Game/Blueprints/Enemies/naranjo/Combat_Interface.Attack`
  (bind _charactermovement (`self.CharacterMovement`))
  (set `CharacterMovementComponent.MaxWalkSpeed` 0.0 _charactermovement)
  (`KismetSystemLibrary.Delay` 2.0)
  (set `CharacterMovementComponent.MaxWalkSpeed` 400.0 _charactermovement))

(event `/Game/Blueprints/Enemies/Damage_Interface.DealDamage`
  (params (Damage :type "Float (double-precision)"))
  (bind _output_get (set `self.HP` (- (`self.HP`) Damage)))
  (`KismetSystemLibrary.PrintString` (`KismetStringLibrary.Conv_DoubleToString` _output_get))
  (if (<= _output_get 0.0)
    (`self.K2_DestroyActor`)))

(fn `UserConstructionScript`)