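; Arbol enemy character driven by arbol_AIController, counted in game-mode totals as regular, mini-boss or boss.
; Attacks play a montage, socket-to-socket sphere traces deal damage with knockback and player hitstop, and a separate event leaps toward the player.
; DealDamage animates a proximity-shown health bar; stun and knockback, computed from attack type, Weight and weapon stats, sit inside its zero-health branch.
; The effects, reputation and destroy death chain is unconnected.
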(event `AttackTrace`
  (bind (_returnvalue_roll _returnvalue_pitch _returnvalue_yaw) (`KismetMathLibrary.BreakRotator` (`self.K2_GetActorRotation`)))
  (bind (_knockback_x _knockback_y _knockback_z) (`KismetMathLibrary.BreakVector` (`self.Knockback`)))
  (bind _mesh (`self.Mesh`))
  (bind (_bsuccess _asvuck_character) (cast `` (`GameplayStatics.GetPlayerCharacter` 0) :!pure true))
  (bind (_returnvalue_x _returnvalue_y) (`KismetMathLibrary.BreakVector` (* (`KismetMathLibrary.GetForwardVector` (`KismetMathLibrary.MakeRotator` 0.0 0.0 _returnvalue_yaw)) _knockback_x)))
  (bind (_outhits _returnvalue) (`KismetSystemLibrary.SphereTraceMultiForObjects` :`Start` (`SceneComponent.GetSocketLocation` _mesh "TraceStart") :`End` (`SceneComponent.GetSocketLocation` _mesh "TraceEnd") :`Radius` 80.0 :`ObjectTypes` (`|MakeArray` "ObjectTypeQuery3" :!type "EObjectTypeQuery Enum") :`DrawTime` 0.5))
  (if _returnvalue
    (for _array_element _outhits
      (if (== (`GameplayStatics.GetObjectClass` (`.HitActor` (`GameplayStatics.BreakHitResult` _array_element))) null)
        (if (not (`KismetArrayLibrary.Array_Contains` (`self.Targets Hit`) (`.HitActor` (`GameplayStatics.BreakHitResult` _array_element))))
          (`KismetArrayLibrary.Array_Add` (`self.Targets Hit`) (`.HitActor` (`GameplayStatics.BreakHitResult` _array_element)))
          (message `/Game/Blueprints/Enemies/arbol/arbol_BP.DealDamage` (`.HitActor` (`GameplayStatics.BreakHitResult` _array_element)) (`self.Attack Damage`) 0 (`self.Attack Stun`) (`KismetMathLibrary.MakeVector` _returnvalue_x _returnvalue_y _knockback_z) (`.ImpactPoint` (`GameplayStatics.BreakHitResult` _array_element)))
          (if (not (<= (`/Game/Blueprints/Enemies/arbol/arbol_BP.Current Health` _asvuck_character) 0.0))
            (`self.StartHitstop` _asvuck_character (`self.Hitstop Duration`)))
          (`KismetSystemLibrary.Delay` 0.2)
          (`KismetArrayLibrary.Array_Clear` (`self.Targets Hit`)))))))

(event `self.Attack`
  (bind _charactermovement (`self.CharacterMovement`))
  (if (<= (`self.Vuck Stun Duration`) 0.0)
    (set `CharacterMovementComponent.MaxWalkSpeed` 0.0 _charactermovement)
    (`|PlayMontage` (`self.Mesh`)
      (:`then`
        (`Controller.StopMovement` (`AIBlueprintHelperLibrary.GetAIController` self)))
      (:`OnCompleted`
        (set `CharacterMovementComponent.MaxWalkSpeed` 900.0 _charactermovement :!label _label))
      (:`OnInterrupted`
        (goto _label)))))

(event `self.ReceiveBeginPlay`
  (bind (_bsuccess _askrashers_game_mode) (cast `` (`GameplayStatics.GetGameMode`) :!pure true))
  (`|ExecutionSequence`
    (:`then_0`
      (if (`self.CountEnemy`)
        (set `/Game/Blueprints/Enemies/arbol/arbol_BP.Enemies Left` (+ (`/Game/Blueprints/Enemies/arbol/arbol_BP.Enemies Left` _askrashers_game_mode) 1) _askrashers_game_mode)))
    (:`then_1`
      (if (`self.MiniBoss`)
        (set `/Game/Blueprints/Enemies/arbol/arbol_BP.MiniBoss Left` (+ (`/Game/Blueprints/Enemies/arbol/arbol_BP.MiniBoss Left` _askrashers_game_mode) 1) _askrashers_game_mode)))
    (:`then_2`
      (if (`self.Boss`)
        (set `/Game/Blueprints/Enemies/arbol/arbol_BP.Boss Left` (+ (`/Game/Blueprints/Enemies/arbol/arbol_BP.Boss Left` _askrashers_game_mode) 1) _askrashers_game_mode)))))

(event `Rotate and Launch`
  (bind _returnvalue (`KismetMathLibrary.MakeRotator` 0.0 0.0 (.yaw (`self.GetControlRotation`))))
  (bind _asvuck_character (cast `` (`GameplayStatics.GetPlayerCharacter` 0)))
  (bind (_returnvalue_roll _returnvalue_pitch _returnvalue_yaw) (`KismetMathLibrary.BreakRotator` (`KismetMathLibrary.FindLookAtRotation` (`self.K2_GetActorLocation`) (`self.K2_GetActorLocation` _asvuck_character))))
  (`self.K2_SetActorRelativeRotation` (`KismetMathLibrary.MakeRotator` 0.0 0.0 _returnvalue_yaw))
  (`self.LaunchCharacter` (`KismetMathLibrary.GreaterGreater_VectorRotator` (0.0 0.0 500.0) _returnvalue) true)
  (`KismetSystemLibrary.Delay` 0.1)
  (`self.LaunchCharacter` (`KismetMathLibrary.GreaterGreater_VectorRotator` (1000.0 0.0 0.0) _returnvalue) true))

(event `Death`
  (bind (_bsuccess _askrashers_game_mode) (cast `` (`GameplayStatics.GetGameMode`) :!pure true))
  (`|ExecutionSequence`
    (:`then_0`
      (if (`self.CountEnemy`)
        (set `/Game/Blueprints/Enemies/arbol/arbol_BP.Enemies Left` (+ (`/Game/Blueprints/Enemies/arbol/arbol_BP.Enemies Left` _askrashers_game_mode) -1) _askrashers_game_mode)))
    (:`then_1`
      (if (`self.MiniBoss`)
        (set `/Game/Blueprints/Enemies/arbol/arbol_BP.MiniBoss Left` (+ (`/Game/Blueprints/Enemies/arbol/arbol_BP.MiniBoss Left` _askrashers_game_mode) -1) _askrashers_game_mode)))
    (:`then_2`
      (if (`self.Boss`)
        (set `/Game/Blueprints/Enemies/arbol/arbol_BP.Boss Left` (+ (`/Game/Blueprints/Enemies/arbol/arbol_BP.Boss Left` _askrashers_game_mode) -1) _askrashers_game_mode)))))

(event `self.DealDamage`
  (params (Damage :type "Float (double-precision)") (Attack :type Integer) (`Stun Duration` :type "Float (double-precision)") (Knockback :type "Vector Structure") (`Hit Location` :type "Vector Structure"))
  (bind _current_health (`self.Current Health`))
  (bind _vuck_stun_duration (`self.Vuck Stun Duration`))
  (bind _current_health_2 (`self.Current Health`))
  (bind _aswbp_health_bar (cast `/Game/ThirdPerson/Blueprints/WBP_HealthBar` (`WidgetComponent.GetUserWidgetObject` (`self.Enemy_Healthbar`)) :!pure true))
  (`self.Damaged`)
  (set `self.Temp HP` _current_health_2)
  (set `self.Current Health` (- _current_health_2 Damage))
  (`|ExecutionSequence`
    (:`then_0`
      (`ProgressBar.SetPercent` (`/Game/ThirdPerson/Blueprints/WBP_HealthBar.Health_progressbar` _aswbp_health_bar) (/ _current_health 70.0))
      (if (<= _current_health 0.0)
        (`/Game/Blueprints/Enemies/arbol/arbol_AIController.Dead` (cast `/Game/Blueprints/Enemies/arbol/arbol_AIController` (`AIBlueprintHelperLibrary.GetAIController` self) :!pure true))
        (`PrimitiveComponent.SetCollisionObjectType` (`self.CapsuleComponent`) "ECC_WorldDynamic")
        (`self.Calculate Stun and Knockback` Attack)
        (if (== (`self.VuckKnockback`) (0.0 0.0 0.0))
          (`self.LaunchCharacter` Knockback true true)
          (set `self.Vuck Stun Duration` `Stun Duration`))
        (if (> (`self.Current Health`) 0.0)
          (if (> (`self.Vuck Stun Duration`) 0.0)
            (bind _asarbol_aicontroller (cast `/Game/Blueprints/Enemies/arbol/arbol_AIController` (`AIBlueprintHelperLibrary.GetAIController` self)))
            (`Controller.StopMovement` _asarbol_aicontroller)
            (`/Game/Blueprints/Enemies/arbol/arbol_AIController.Stunned` _asarbol_aicontroller _vuck_stun_duration)
            (if (> _vuck_stun_duration 0.0) :!label _label_2
              (`KismetSystemLibrary.RetriggerableDelay` 0.1)
              (set `self.Vuck Stun Duration` (- _vuck_stun_duration 0.1))
              (goto _label_2))))))
    (:`then_1`
      (bind (_direction _hp_loss) (`Timeline|TL_HPLoss` :!via `PlayFromStart`)
        (:`Update`
          (`ProgressBar.SetPercent` (`/Game/ThirdPerson/Blueprints/WBP_HealthBar.Health_progressbar` _aswbp_health_bar) (/ (- (`self.Temp HP`) (* Damage _hp_loss)) 70.0)))))))

(event `self.OnLanded`
  (params (Hit :type "HitResult Structure (by ref)"))
  (`NiagaraFunctionLibrary.SpawnSystemAtLocation` null (`SceneComponent.K2_GetComponentLocation` (`self.SmokeParticles`)) (struct) (0.75 0.75 0.75)))

(event `self.HealthbarTrigger.OnComponentBeginOverlap`
  (params (OverlappedComponent :type "PrimitiveComponent Object Reference") (OtherActor :type "Actor Object Reference") (OtherComp :type "PrimitiveComponent Object Reference") (OtherBodyIndex :type Integer) (bFromSweep :type Boolean) (SweepResult :type "HitResult Structure (by ref)"))
  (if (== OtherActor (`GameplayStatics.GetPlayerCharacter` 0))
    (`SceneComponent.SetVisibility` (`self.Enemy_Healthbar`) true false)))

(event `self.HealthbarTrigger.OnComponentEndOverlap`
  (params (OverlappedComponent :type "PrimitiveComponent Object Reference") (OtherActor :type "Actor Object Reference") (OtherComp :type "PrimitiveComponent Object Reference") (OtherBodyIndex :type Integer))
  (if (and (== (`GameplayStatics.GetPlayerCharacter` 0) OtherActor) (not (`self.Recently Damaged`)))
    (`SceneComponent.SetVisibility` (`self.Enemy_Healthbar`) false false :!label _label_3)))

(event `Damaged`
  (`GameplayStatics.SpawnSoundAttached` (`self.SihnHurtSound`) (`self.Mesh`) "None" (0.0 0.0 0.0) (struct) "KeepRelativeOffset" true 0.7 1.0 0.0 null null)
  (set `self.Recently Damaged` true)
  (`SceneComponent.SetVisibility` (`self.Enemy_Healthbar`) true false)
  (`KismetSystemLibrary.RetriggerableDelay` 3.0)
  (set `self.Recently Damaged` false)
  (goto _label_3))

(fn `NewFunction`
  (params (`As WBP Health Bar_0` :type "/Game/ThirdPerson/Blueprints/WBP_HealthBar Object Reference"))
  (set `self.As WBP Health Bar_0` `As WBP Health Bar_0`))

(fn `UserConstructionScript`
  (set `CharacterMovementComponent.MaxWalkSpeed` (`self.Speed`) (`self.CharacterMovement`))
  (switch `int` (`KismetMathLibrary.RandomIntegerInRange` 0 2)
    (:`0`
      (set `self.SihnAttackSound` null)
      (set `self.SihnDeathSound` null)
      (set `self.SihnHurtSound` null))
    (:`1`
      (set `self.SihnAttackSound` null)
      (set `self.SihnDeathSound` null)
      (set `self.SihnHurtSound` null))
    (:`2`
      (set `self.SihnAttackSound` null)
      (set `self.SihnDeathSound` null)
      (set `self.SihnHurtSound` null))))