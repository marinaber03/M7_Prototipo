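; BP_CharacterWASD is a player character with axis-driven movement, mouse-style look, sprinting and camera zoom.
; Movement follows control-rotation yaw, while turn and look axes feed controller yaw and pitch.
; Sprint switches max walk speed between SprintSpeed and WalkSpeed, playing a world camera shake while held and stopping all shakes on release.
; The zoom axis adjusts spring arm length by ZoomAmount without clamping.
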(event `self.ReceiveTick`
  (params (DeltaSeconds :type "Float (single-precision)")))

(event `InputAxis|FordwardAxis`
  (params (AxisValue :type "Float (single-precision)"))
  ; Movement
  (`self.AddMovementInput` (`KismetMathLibrary.GetForwardVector` (`KismetMathLibrary.MakeRotator` 0.0 0.0 (.yaw (`self.GetControlRotation`)))) AxisValue))

(event `InputAxis|Turn`
  (params (AxisValue :type "Float (single-precision)"))
  ; Turn
  (`self.AddControllerYawInput` AxisValue))

(event `InputAxis|LookUp`
  (params (AxisValue :type "Float (single-precision)"))
  ; Turn
  (`self.AddControllerPitchInput` AxisValue))

(event `InputAxis|HorizontalAxis`
  (params (AxisValue :type "Float (single-precision)"))
  ; Movement
  (`self.AddMovementInput` (`KismetMathLibrary.GetRightVector` (`KismetMathLibrary.MakeRotator` 0.0 0.0 (.yaw (`self.GetControlRotation`)))) AxisValue))

(event `InputAction|Sprint`
  (params (Key :type "Key Structure"))
  ; CameraShake
  (:`Pressed`
    (`GameplayStatics.PlayWorldCameraShake` "/Game/Blueprints/BP_CameraShakeSprint.BP_CameraShakeSprint_C" (`self.K2_GetActorLocation`) 0.0 600.0)
    ; Sprint
    (set `CharacterMovementComponent.MaxWalkSpeed` (`self.SprintSpeed`) (`self.CharacterMovement`)))
  (:`Released`
    (`PlayerCameraManager.StopAllCameraShakes` (`GameplayStatics.GetPlayerCameraManager` 0) true)
    (set `CharacterMovementComponent.MaxWalkSpeed` (`self.WalkSpeed`) (`self.CharacterMovement`))))

(event `InputAxis|CameraZoom`
  (params (AxisValue :type "Float (single-precision)"))
  (bind _springarm (`self.springArm`))
  ; Zoom
  (set `SpringArmComponent.TargetArmLength` (+ (* AxisValue (`self.ZoomAmount`)) (`SpringArmComponent.TargetArmLength` _springarm)) _springarm))

(fn `UserConstructionScript`)