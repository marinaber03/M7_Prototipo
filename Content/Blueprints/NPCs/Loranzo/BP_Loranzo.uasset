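; Loranzo NPC that makes a smoke-and-sound entrance, plays a montage, then starts its AI when the montage completes.
; The entrance runs on BeginPlay, and a one-time InteractionRadius overlap feeds the same sequence when HostelMission is off.
; DealDamage destroys the actor immediately with an effect and sound.
; With HostelMission set, the construction script calls ProgrammedDeath.
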(event `self.InteractionRadius.OnComponentBeginOverlap`
  (params (OverlappedComponent :type "PrimitiveComponent Object Reference") (OtherActor :type "Actor Object Reference") (OtherComp :type "PrimitiveComponent Object Reference") (OtherBodyIndex :type Integer) (bFromSweep :type Boolean) (SweepResult :type "HitResult Structure (by ref)"))
  (bind _returnvalue (`SceneComponent.K2_GetComponentLocation` (`self.SmokeParticles`)))
  (if (and (== (`GameplayStatics.GetObjectClass` OtherActor) null) (not (`self.HostelMission`)))
    (`/Engine/EditorBlueprintResources/StandardMacros.DoOnce` false
      (:`Completed`
        (`NiagaraFunctionLibrary.SpawnSystemAtLocation` null _returnvalue :!label _label)
        (`GameplayStatics.SpawnSoundAtLocation` null _returnvalue (struct) 1.0 1.0 0.0 null null)
        (`|PlayMontage` (`self.Mesh`)
          (:`OnCompleted`
            (`self.StartAI` (`.AsBistro AIController` (cast `` _ :!pure true)))))))))

(event `self.ReceiveBeginPlay`
  (goto _label))

(event `self.DealDamage`
  (params (Damage :type "Float (double-precision)") (Attack :type Integer) (`Stun Duration` :type "Float (double-precision)") (Knockback :type "Vector Structure") (`Hit Location` :type "Vector Structure"))
  (bind _returnvalue (`self.K2_GetActorLocation`))
  (`NiagaraFunctionLibrary.SpawnSystemAtLocation` null _returnvalue (struct) (0.75 0.75 0.75))
  (`GameplayStatics.SpawnSoundAtLocation` null _returnvalue (struct) 2.0 1.0 0.0 null null)
  (`self.K2_DestroyActor`))

(fn `UserConstructionScript`
  (if (`self.HostelMission`)
    (`self.Programmed Death`)))