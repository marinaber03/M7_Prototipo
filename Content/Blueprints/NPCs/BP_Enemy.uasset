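; BP_Enemy is an enemy NPC with a health component and a widget-component health bar that appears when the player is near.
; On BeginPlay it hides the bar and hands its health component to the WBP_HealthBar widget.
; A sphere overlap with BP_Char_SrLemonin shows or hides the bar.
; Tick polls the health component's IsDead flag and destroys the actor once it is set.
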(event `self.ReceiveBeginPlay`
  (bind _widgetcomponent (`self.WidgetComponent`))
  (`SceneComponent.SetVisibility` _widgetcomponent false false)
  (bind _aswbp_health_bar (cast `/Game/SirLemonin/Blueprints/WBP_HealthBar` (`WidgetComponent.GetWidget` _widgetcomponent)))
  (set `/Game/SirLemonin/Blueprints/WBP_HealthBar.Healthcomp` (`self.BP_HealthComponent`) _aswbp_health_bar))

(event `self.ReceiveTick`
  (params (DeltaSeconds :type "Float (single-precision)"))
  (if (`/Game/SirLemonin/Blueprints/BP_HealthComponent.isDead` (`self.BP_HealthComponent`))
    (`self.K2_DestroyActor`)))

(event `self.Sphere.OnComponentBeginOverlap`
  (params (OverlappedComponent :type "PrimitiveComponent Object Reference") (OtherActor :type "Actor Object Reference") (OtherComp :type "PrimitiveComponent Object Reference") (OtherBodyIndex :type Integer) (bFromSweep :type Boolean) (SweepResult :type "HitResult Structure (by ref)"))
  (cast `/Game/SirLemonin/Blueprints/BP_Char_SrLemonin` OtherActor)
  (`SceneComponent.SetVisibility` (`self.WidgetComponent`) true false))

(event `self.Sphere.OnComponentEndOverlap`
  (params (OverlappedComponent :type "PrimitiveComponent Object Reference") (OtherActor :type "Actor Object Reference") (OtherComp :type "PrimitiveComponent Object Reference") (OtherBodyIndex :type Integer))
  (cast `/Game/SirLemonin/Blueprints/BP_Char_SrLemonin` OtherActor)
  (`SceneComponent.SetVisibility` (`self.WidgetComponent`) false false))

(fn `UserConstructionScript`)