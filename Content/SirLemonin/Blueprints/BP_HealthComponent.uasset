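; BP_HealthComponent is a health component that tracks hit points and death state for its owner.
; BeginPlay sets maximum and current health to full.
; ReceiveDamage ignores hits once dead, otherwise subtracts damage, clamping health to zero and setting IsDead when it would reach zero or below.
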(event `self.ReceiveBeginPlay`
  (set `self.MaxHP` 100.0)
  (set `self.CurrentHP` 100.0))

(fn `ReceiveDamage`
  (params (damage :type "Float (double-precision)" :default 20.0))
  (bind _returnvalue (- (`self.CurrentHP`) damage))
  (if (not (`self.isDead`))
    (if (<= _returnvalue 0.0)
      (set `self.CurrentHP` 0.0)
      (set `self.isDead` true)
      (else
        (set `self.CurrentHP` _returnvalue)))))